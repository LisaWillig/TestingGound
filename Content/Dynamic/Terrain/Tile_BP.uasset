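; Terrain tile Blueprint for an infinite terrain system, with a one-way style barrier, spawn trigger and self-cleanup.
; The barrier starts green and passable; when an actor overlap ends and the player is outside BarrierCollision, it turns red and solid and InfiniteTerrain_GM runs SpawnFunction.
; An overlap beginning with the player inside DeleteTilesCollision destroys the tile.
; GetAttachLocation exposes the Arrow's world transform as an attach point.
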(event EventBeginPlay
  (CallFunction|UnlockBarrier))

(event Collision|EventActorEndOverlap
  (params (OtherActor :type Actor%20Object%20Reference))
  (if (Collision|IsOverlappingActor (Variables|Default|GetBarrierCollision) (Game|Player|GetPlayerPawn 0) :!class /Script/Engine.PrimitiveComponent)
    (CallFunction|UnlockBarrier)
    (else
      (CallFunction|LockBarrier)
      (bind _asinfinite_terrain_gm (Utilities|Casting|CastToInfiniteTerrain_GM (Game|GetGameMode)))
      (Default|SpawnFunction _asinfinite_terrain_gm))))

(event Collision|EventActorBeginOverlap
  (params (OtherActor :type Actor%20Object%20Reference))
  (if (Collision|IsOverlappingActor (Variables|Default|GetDeleteTilesCollision) (Game|Player|GetPlayerPawn 0) :!class /Script/Engine.PrimitiveComponent)
    (Actor|DestroyActor (Components|GetOwner (Variables|Default|GetDeleteTilesCollision)))))

(fn ConstructionScript)

(fn GetAttachLocation
  (return (Transformation|GetWorldTransform (Variables|Default|GetArrow))))

(fn UnlockBarrier
  (Collision|SetCollisionEnabled (Variables|Default|GetBarrier) "NoCollision")
  (Rendering|Material|SetMaterial (Variables|Default|GetBarrier) 0 "/Game/Dynamic/Terrain/GreenBarrier.GreenBarrier"))

(fn LockBarrier
  (Collision|SetCollisionEnabled (Variables|Default|GetBarrier) "QueryAndPhysics")
  (Rendering|Material|SetMaterial (Variables|Default|GetBarrier) 0 "/Game/Dynamic/Terrain/RedBarrier.RedBarrier"))