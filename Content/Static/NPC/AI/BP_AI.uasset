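; AI controller for a guard NPC that runs the guard behavior tree on the patrol blackboard.
; AI perception updates feed the blackboard's enemy key: a sensed actor is stored as the target, and a failed sense clears it.
; Actors tagged "Enemy" are ignored, so the guard only targets actors without that tag.
; The aiming and shooting function is an empty stub.
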(event OnTargetPerceptionUpdated(AIPerception)
  (params (Actor :type Actor%20Object%20Reference) (Stimulus :type AI%20Stimulus%20Structure))
  (CallFunction|PreceiveEnemy Actor Stimulus Actor))

(event EventBeginPlay
  (bind _blackboardcomponent (Class|AIController|UseBlackboard "/Game/Static/NPC/AI/BB_Patrol.BB_Patrol"))
  (AI|RunBehaviorTree "/Game/Static/NPC/AI/BT_GuardBehaviour.BT_GuardBehaviour")
  (Variables|Default|SetBlackboradComp _blackboardcomponent))

(fn ConstructionScript)

(fn SetAimingandShooting)

(fn PreceiveEnemy
  (params (ObjectValue :type Object%20Object%20Reference) (AIStimulus :type AI%20Stimulus%20Structure%20%28by%20ref%29) (self2 :type Actor%20Object%20Reference))
  (if (not (Actor|ActorHasTag self2 "Enemy"))
    (if (.bSuccessfullySensed (Utilities|Struct|BreakAIStimulus AIStimulus))
      (AI|Components|Blackboard|SetValueasObject (Variables|Default|GetBlackboradComp) (Variables|Default|GetEnemyKey) ObjectValue)
      (else
        (AI|Components|Blackboard|ClearValue (Variables|Default|GetBlackboradComp) (Variables|Default|GetEnemyKey))))))