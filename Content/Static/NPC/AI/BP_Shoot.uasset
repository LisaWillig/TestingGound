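; Behavior tree task that makes an AI-controlled BP_TPCharacter aim and shoot at a target.
; On execute it sets the pawn's Aiming and Shooting flags and focuses the controller on the actor from the Target blackboard key.
; It never finishes execution itself, so it runs until aborted, then resets both flags, clears focus and finishes the abort.
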(event EventReceiveExecuteAI
  (params (OwnerController :type AI%20Controller%20Object%20Reference) (ControlledPawn :type Pawn%20Object%20Reference))
  (bind _asbp_tpcharacter (Utilities|Casting|CastToBP_TPCharacter ControlledPawn))
  (Variables|/Game/Static/NPC/Character/TP_Char/BP_TPCharacter.BP_TPCharacter_C|SetAiming _asbp_tpcharacter true)
  (Variables|/Game/Static/NPC/Character/TP_Char/BP_TPCharacter.BP_TPCharacter_C|SetShooting _asbp_tpcharacter true)
  (AI|SetFocus OwnerController (AI|BehaviorTree|GetBlackboardValueasActor (Variables|Default|GetTarget))))

(event EventReceiveAbortAI
  (params (OwnerController :type AI%20Controller%20Object%20Reference) (ControlledPawn :type Pawn%20Object%20Reference))
  (bind _asbp_tpcharacter (Utilities|Casting|CastToBP_TPCharacter ControlledPawn))
  (Variables|/Game/Static/NPC/Character/TP_Char/BP_TPCharacter.BP_TPCharacter_C|SetAiming _asbp_tpcharacter false)
  (Variables|/Game/Static/NPC/Character/TP_Char/BP_TPCharacter.BP_TPCharacter_C|SetShooting _asbp_tpcharacter false)
  (AI|ClearFocus OwnerController)
  (Class|BTTaskBlueprintBase|FinishAbort))