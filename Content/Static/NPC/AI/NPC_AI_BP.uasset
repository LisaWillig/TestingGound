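; AI controller for guard NPCs that runs the GuardBehaviour behavior tree on the Patrol blackboard.
; AI perception writes sensed actors without the "Enemy" tag to EnemyKey and clears the key when one is no longer sensed.
; Each tick, it sets the controlled ThirdPersonCharacter's Aiming flag according to whether the controller has a valid focus actor.
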(event OnTargetPerceptionUpdated(AIPerception)
  (params (Actor :type Actor%20Object%20Reference) (Stimulus :type AI%20Stimulus%20Structure))
  (if (not (Actor|ActorHasTag Actor "Enemy"))
    (if (.bSuccessfullySensed (Utilities|Struct|BreakAIStimulus Stimulus))
      (AI|Components|Blackboard|SetValueasObject (Variables|Default|GetBlackboradComp) (Variables|Default|GetEnemyKey) Actor)
      (else
        (AI|Components|Blackboard|ClearValue (Variables|Default|GetBlackboradComp) (Variables|Default|GetEnemyKey))))))

(event EventBeginPlay
  (bind _blackboardcomponent (Class|AIController|UseBlackboard "/Game/Static/NPC/AI/Patrol.Patrol"))
  (AI|RunBehaviorTree "/Game/Static/NPC/AI/GuardBehaviour.GuardBehaviour")
  (Variables|Default|SetBlackboradComp _blackboardcomponent))

(event EventTick
  (params (DeltaSeconds :type Float%20%28single-precision%29))
  (bind _asthird_person_character (Utilities|Casting|CastToThirdPersonCharacter (Pawn|GetControlledPawn)))
  (Variables|/Game/Static/NPC/Behaviour/ThirdPersonCharacter.ThirdPersonCharacter_C|SetAiming _asthird_person_character (Utilities|IsValid (Class|AIController|GetFocusActor))))

(fn ConstructionScript)